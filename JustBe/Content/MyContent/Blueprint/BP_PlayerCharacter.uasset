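; Player character for a side-scrolling action game, with sprite-flip movement, jumping, directional melee attacks and a mask-driven ability.
; Attacks pick up, down or forward from vertical input and damage via a box trace; the Dash Launcher mask ability sweeps along a timeline, damaging and launching the first enemy hit upward with the player.
; BPCStats supplies combat stats and stamina, which regenerates by timer after a delay.
; AddXP handles leveling and updates the HUD.
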(event `self.ReceiveBeginPlay`
  (bind _bpc_stats (`self.BPC_Stats`))
  (`EnhancedInputSubsystemInterface.AddMappingContext` (pcsubsystem `EnhancedInputLocalPlayerSubsystem` (`GameplayStatics.GetPlayerController` 0)) "/Game/MyContent/Input/IMC_MainCharacter.IMC_MainCharacter" 0 (struct))
  (bind _returnvalue (`|CreateWidget` "/Game/MyContent/Blueprint/UI/WBP_HUD.WBP_HUD_C"))
  (bind _output_get (set `self.HUDRef` _returnvalue))
  (`UserWidget.AddToViewport` _output_get 0)
  (`/Game/MyContent/Blueprint/UI/WBP_HUD.UpdateXPUI` _output_get (`/Game/MyContent/Blueprint/Struct/BPC_Stats.CurrentXP` _bpc_stats) (`/Game/MyContent/Blueprint/Struct/BPC_Stats.MaxXP` _bpc_stats) (`KismetMathLibrary.FTrunc` (`/Game/MyContent/Blueprint/Struct/BPC_Stats.CurrentLevel` _bpc_stats))))

(event `EnhancedInput|/Game/MyContent/Input/Actions/IA_Move`
  (params (ActionValue :type "Float (double-precision)") (ElapsedSeconds :type "Float (double-precision)") (TriggeredSeconds :type "Float (double-precision)") (InputAction :type "InputAction Object Reference" :default "/Game/MyContent/Input/Actions/IA_Move.IA_Move"))
  (:`Triggered`
    (`self.AddMovementInput` (1.0 0.0 0.0) ActionValue)
    (if (> ActionValue 0.0)
      (`SceneComponent.SetRelativeScale3D` (`self.Sprite`) (1.0 1.0 1.0))
      (elif (< ActionValue 0.0)
        (`SceneComponent.SetRelativeScale3D` (`self.Sprite`) (-1.0 1.0 1.0))))))

(event `EnhancedInput|/Game/MyContent/Input/Actions/IA_Jump`
  (params (ActionValue :type Boolean) (ElapsedSeconds :type "Float (double-precision)") (TriggeredSeconds :type "Float (double-precision)") (InputAction :type "InputAction Object Reference" :default "/Game/MyContent/Input/Actions/IA_Jump.IA_Jump"))
  (:`Started`
    (`self.Jump`))
  (:`Completed`
    (`self.StopJumping`)))

(event `EnhancedInput|/Game/MyContent/Input/Actions/IA_VerticalAttack`
  (params (ActionValue :type "Float (double-precision)") (ElapsedSeconds :type "Float (double-precision)") (TriggeredSeconds :type "Float (double-precision)") (InputAction :type "InputAction Object Reference" :default "/Game/MyContent/Input/Actions/IA_VerticalAttack.IA_VerticalAttack"))
  (:`Triggered`
    (set `self.VerticalInput` ActionValue))
  (:`Completed`
    (set `self.VerticalInput` 0.0)))

(event `EnhancedInput|/Game/MyContent/Input/Actions/IA_Attack`
  (params (ActionValue :type Boolean) (ElapsedSeconds :type "Float (double-precision)") (TriggeredSeconds :type "Float (double-precision)") (InputAction :type "InputAction Object Reference" :default "/Game/MyContent/Input/Actions/IA_Attack.IA_Attack"))
  (:`Started`
    (if (`self.bCanAttack`)
      (if (not (<= (`/Game/MyContent/Blueprint/Struct/BPC_Stats.CurrentStamina` (`self.BPC_Stats`)) 4.0))
        (`self.ConsumeStaminaAndPauseRegen` 5.0)
        (set `self.bCanAttack` false)
        (if (> (`self.VerticalInput`) 0.3)
          (`self.PerformAttack` (0.0 0.0 120.0) (struct :`Pitch` 90.0))
          (elif (< (`self.VerticalInput`) -0.3)
            (`self.PerformAttack` (0.0 0.0 -100.0) (struct :`Pitch` -90.0))
            (else
              (`self.PerformAttack` (100.0 0.0 0.0) (struct)))))
        (`KismetSystemLibrary.Delay` (`/Game/MyContent/Blueprint/Struct/BPC_Stats.CurrentAttackCooldown` (`self.BPC_Stats`)))
        (set `self.bCanAttack` true)))))

(event `EnhancedInput|/Game/MyContent/Input/Actions/IA_Ability`
  (params (ActionValue :type Boolean) (ElapsedSeconds :type "Float (double-precision)") (TriggeredSeconds :type "Float (double-precision)") (InputAction :type "InputAction Object Reference" :default "/Game/MyContent/Input/Actions/IA_Ability.IA_Ability"))
  (bind _currentmask (`/Game/MyContent/Blueprint/Struct/BPC_MaskSystem.CurrentMask` (`self.BPC_MaskSystem`)))
  (:`Started`
    (`/Engine/EditorBlueprintResources/StandardMacros.IsValid` _currentmask
      (:`Is Valid`
        (switch `/Game/MyContent/Blueprint/Struct/E_MaskAbilityType` (`/Game/MyContent/Blueprint/Struct/PDA_MaskData.AbilityType` _currentmask)
          (:`NewEnumerator0`
            (if (`self.bCanDoDash`)
              (set `self.bCanDoDash` false)
              (`self.ExecuteDashLauncher`)
              (`KismetSystemLibrary.Delay` 0.5)
              (set `self.bCanDoDash` true))))))))

(event `ExecuteDashLauncher`
  (bind _returnvalue (`self.K2_GetActorLocation`))
  (bind _relativescale3d_x (`KismetMathLibrary.BreakVector` (`SceneComponent.RelativeScale3D` (`self.Sprite`))))
  (bind _returnvalue_2 (`KismetMathLibrary.MakeVector` _relativescale3d_x))
  (if (not (<= (`/Game/MyContent/Blueprint/Struct/BPC_Stats.CurrentStamina` (`self.BPC_Stats`)) 19.0))
    (`self.ConsumeStaminaAndPauseRegen` 20.0)
    (set `self.bHasHitEnemy` false)
    (bind _output_get (set `self.DashStartLocation` (`self.K2_GetActorLocation`)))
    (set `self.DashDirection` _returnvalue_2)
    (set `self.DashEndLocation` (+ _output_get (* _returnvalue_2 (`self.AbilityDashLength`))))
    (bind (_direction _alpha) (`Timeline|TL_Dash` :!via `PlayFromStart`)
      (:`Update`
        (`self.K2_SetActorLocation` (`KismetMathLibrary.VLerp` (`self.DashStartLocation`) (`self.DashEndLocation`) _alpha) true)
        (bind _outhit (`KismetSystemLibrary.BoxTraceSingle` :`Start` _returnvalue :`End` (+ _returnvalue (* (`self.DashDirection`) 20.0)) :`HalfSize` (30.0 30.0 60.0) :`TraceChannel` "TraceTypeQuery1" :`DrawDebugType` "ForDuration"))
        (bind _asbp_enemy (cast `/Game/MyContent/Blueprint/Enemies/BP_Enemy` (`.HitActor` (`GameplayStatics.BreakHitResult` _outhit))))
        (if (not (`self.bHasHitEnemy`))
          (set `self.bHasHitEnemy` true)
          (`TimelineComponent.Stop` (`self.TL_Dash`))
          (`GameplayStatics.ApplyDamage` _asbp_enemy (`self.AbilityDashDamage`))
          (`self.LaunchCharacter` (0.0 0.0 1000.0) true true)
          (`self.LaunchCharacter` _asbp_enemy (0.0 0.0 800.0) false true))))))

(event `StartStaminaRegene`
  (bind _returnvalue (`KismetSystemLibrary.K2_SetTimerDelegate` (delegate `RegenStamina`) 0.1 true))
  (set `self.StaminaTimerHandle` _returnvalue))

(event `RegenStamina`
  (bind _bpc_stats (`self.BPC_Stats`))
  (bind _currentstamina (`/Game/MyContent/Blueprint/Struct/BPC_Stats.CurrentStamina` _bpc_stats))
  (bind _maxstamina (`/Game/MyContent/Blueprint/Struct/BPC_Stats.MaxStamina` _bpc_stats))
  (if (< _currentstamina _maxstamina)
    (set `/Game/MyContent/Blueprint/Struct/BPC_Stats.CurrentStamina` (`KismetMathLibrary.FClamp` (+ _currentstamina 0.5) 0.0 _maxstamina) _bpc_stats)
    (else
      (`KismetSystemLibrary.K2_ClearAndInvalidateTimerHandle` (`self.StaminaTimerHandle`)))))

(event `ConsumeStaminaAndPauseRegen`
  (params (StaminaToConsume :type "Float (double-precision)"))
  (bind _bpc_stats (`self.BPC_Stats`))
  (set `/Game/MyContent/Blueprint/Struct/BPC_Stats.CurrentStamina` (- (`/Game/MyContent/Blueprint/Struct/BPC_Stats.CurrentStamina` _bpc_stats) StaminaToConsume) _bpc_stats)
  (`KismetSystemLibrary.K2_ClearAndInvalidateTimerHandle` (`self.StaminaTimerHandle`))
  (`KismetSystemLibrary.Delay` 1.0)
  (`self.StartStaminaRegene`))

(event `AddXP`
  (params (XPAmount :type "Float (double-precision)"))
  (bind _bpc_stats (`self.BPC_Stats`))
  (bind _bpc_stats_2 (`self.BPC_Stats`))
  (bind _bpc_stats_3 (`self.BPC_Stats`))
  (bind _returnvalue (+ XPAmount (`/Game/MyContent/Blueprint/Struct/BPC_Stats.CurrentXP` _bpc_stats_2)))
  (if (>= _returnvalue (`/Game/MyContent/Blueprint/Struct/BPC_Stats.MaxXP` _bpc_stats_2))
    (set `/Game/MyContent/Blueprint/Struct/BPC_Stats.CurrentExp` (- (`/Game/MyContent/Blueprint/Struct/BPC_Stats.CurrentXP` _bpc_stats_3) (`/Game/MyContent/Blueprint/Struct/BPC_Stats.MaxXP` _bpc_stats_3)) _bpc_stats_3)
    (set `/Game/MyContent/Blueprint/Struct/BPC_Stats.CurrentLevel` (+ (`/Game/MyContent/Blueprint/Struct/BPC_Stats.CurrentLevel` _bpc_stats_3) 1.0) _bpc_stats_3)
    (else
      (bind _output_get (set `/Game/MyContent/Blueprint/Struct/BPC_Stats.CurrentExp` _returnvalue _bpc_stats))))
  (`/Game/MyContent/Blueprint/UI/WBP_HUD.UpdateXPUI` (`self.HUDRef`) _output_get (`/Game/MyContent/Blueprint/Struct/BPC_Stats.MaxXP` _bpc_stats) (`KismetMathLibrary.FTrunc` (`/Game/MyContent/Blueprint/Struct/BPC_Stats.CurrentLevel` _bpc_stats_2))))

(fn `PerformAttack`
  (params (AttackOffset :type "Vector Structure") (VFXRotation :type "Rotator Structure"))
  (bind _relativescale3d_x (`KismetMathLibrary.BreakVector` (`SceneComponent.RelativeScale3D` (`self.Sprite`))))
  (bind _output_get (set `self.HitLocation` (+ (`KismetMathLibrary.MakeVector` (* (.x AttackOffset) _relativescale3d_x) (.y AttackOffset) (.z AttackOffset)) (`self.K2_GetActorLocation`))))
  (`NiagaraFunctionLibrary.SpawnSystemAtLocation` "/Game/LevelPrototyping/Interactable/JumpPad/Assets/NS_JumpPad.NS_JumpPad" _output_get VFXRotation)
  (bind _outhit (`KismetSystemLibrary.BoxTraceSingle` :`Start` _output_get :`End` _output_get :`HalfSize` (150.0 150.0 50.0) :`Orientation` VFXRotation :`TraceChannel` "TraceTypeQuery1" :`DrawDebugType` "ForDuration"))
  (for _array_element (`|MakeArray` _outhit)
    (`GameplayStatics.ApplyDamage` (`.HitActor` (`GameplayStatics.BreakHitResult` _array_element)) (`/Game/MyContent/Blueprint/Struct/BPC_Stats.CurrentAttackPower` (`self.BPC_Stats`)) (`GameplayStatics.GetPlayerController` 0) self)))

(fn `UserConstructionScript`)