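; BP_Villager is an interactable quest-giver NPC that the player must first color by spending CurrentLevel.
; Interacting with a colored quest villager opens a dialogue widget with text selected by QuestState; other interactions go to the color payment.
; AcceptQuest registers the quest, while ClaimReward grants XP to CurrentLevel, adds a mask and collapses the tracker.
; The quest completion check and ColorChange call are disconnected, so nothing here sets the ready-to-reward state.
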(event `AcceptQuest`
  (bind (_villagerquest_questid _villagerquest_questname _villagerquest_description) (break `/Game/MyContent/Blueprint/Struct/ST_Quest` (`self.VillagerQuest`)))
  (`/Game/MyContent/Blueprint/BP_PlayerCharacter.AddQuest` (`self.PlayerRef`) (`self.VillagerQuest`))
  (set `self.QuestState` "NewEnumerator1")
  (`KismetSystemLibrary.PrintString` (`KismetTextLibrary.Conv_TextToString` _villagerquest_description) true true (struct :`G` 0.66 :`B` 1.0 :`A` 1.0) 7787878788778.0))

(event `/Game/MyContent/Blueprint/Struct/BPI_Interactable.Interact`
  (params (Instigator :type "Actor Object Reference"))
  (bind _returnvalue (`GameplayStatics.GetPlayerController` 0))
  (bind (_villagerquest_questid _villagerquest_questname _villagerquest_description) (break `/Game/MyContent/Blueprint/Struct/ST_Quest` (`self.VillagerQuest`)))
  (bind _bpc_stats (`/Game/MyContent/Blueprint/BP_PlayerCharacter.BPC_Stats` (`self.PlayerRef`)))
  (bind _asbp_player_character (cast `/Game/MyContent/Blueprint/BP_PlayerCharacter` Instigator))
  (set `self.PlayerRef` _asbp_player_character)
  (if (`self.IsColored`)
    (if (`self.HasQuest`)
      (bind _returnvalue_2 (`|CreateWidget` "/Game/MyContent/Blueprint/UI/WBP_VillagerDialogue.WBP_VillagerDialogue_C" null self (`self.QuestState`)))
      (`/Game/MyContent/Blueprint/UI/WBP_VillagerDialogue.SetupDialogue` _returnvalue_2 "Paesano" (select `/Game/MyContent/Blueprint/Struct/E_QuestState` (`self.QuestState`) :`NewEnumerator0` _villagerquest_description :`NewEnumerator1` "Did you finish yet? oh it doesn't seem so" :`NewEnumerator2` "Great, thank you! Here your reward" :`NewEnumerator3` "It looks so beatiful here") "/Game/MyContent/Sprites/Villagers/Sprite1.Sprite1" "NewEnumerator0")
      (`WidgetBlueprintLibrary.SetInputMode_UIOnlyEx` _returnvalue _returnvalue_2)
      (set `PlayerController.bShowMouseCursor` true _returnvalue)
      (`UserWidget.AddToViewport` _returnvalue_2 0)
      (else
        (if (>= (`/Game/MyContent/Blueprint/Struct/BPC_Stats.CurrentLevel` _bpc_stats) (`self.ColorCost`)) :!label _label
          (set `/Game/MyContent/Blueprint/Struct/BPC_Stats.CurrentLevel` (- (`/Game/MyContent/Blueprint/Struct/BPC_Stats.CurrentLevel` _bpc_stats) (`self.ColorCost`)) _bpc_stats)
          (set `self.IsColored` true)
          (`KismetSystemLibrary.PrintString` "Grazie per avermi ridato i colori!")
          (else
            (`KismetSystemLibrary.PrintString` "Non hai abbastanza colori")))))
    (else
      (goto _label))))

(event `ClaimReward`
  (bind _playerref (`self.PlayerRef`))
  (bind _bpc_stats (`/Game/MyContent/Blueprint/BP_PlayerCharacter.BPC_Stats` (`self.PlayerRef`)))
  (set `/Game/MyContent/Blueprint/Struct/BPC_Stats.CurrentLevel` (+ (`/Game/MyContent/Blueprint/Struct/BPC_Stats.CurrentLevel` _bpc_stats) (`.RewardXP_17_649B7628488FBA35C8CB9C8835F1EC58` (break `/Game/MyContent/Blueprint/Struct/ST_Quest` (`self.VillagerQuest`)))) _bpc_stats)
  (set `self.QuestState` "NewEnumerator3")
  (`KismetSystemLibrary.PrintString` "Ecoo la tua ricompensa")
  (`KismetArrayLibrary.Array_Add` (`/Game/MyContent/Blueprint/BP_PlayerCharacter.MaskInventory` _playerref) (`.RewardMask_20_2CDDE6774D8F417EAAE5C1BC4188AF6B` (break `/Game/MyContent/Blueprint/Struct/ST_Quest` (`self.VillagerQuest`))))
  (`Widget.SetVisibility` (`/Game/MyContent/Blueprint/UI/WBP_HUD.WBP_QuestTracker` (`/Game/MyContent/Blueprint/BP_PlayerCharacter.HUDRef` _playerref)) "Collapsed"))

(fn `UserConstructionScript`)