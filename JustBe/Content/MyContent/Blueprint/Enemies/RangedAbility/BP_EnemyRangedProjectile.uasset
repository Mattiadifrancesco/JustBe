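; Projectile for the ranged enemy that bursts on impact, damaging what is nearby.
; On collision hit it spawns an impact Niagara effect, applies radial damage, also damages the player directly if within the same radius, then destroys itself.
; Damage comes from the first BP_Enemy_Ranged found in the world rather than its owner.
; An owner-hit filter and a debug sphere are present but never run.
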(event `self.Collision.OnComponentHit`
  (params (HitComponent :type "PrimitiveComponent Object Reference") (OtherActor :type "Actor Object Reference") (OtherComp :type "PrimitiveComponent Object Reference") (NormalImpulse :type "Vector Structure") (Hit :type "HitResult Structure (by ref)"))
  (bind _returnvalue (`self.K2_GetActorLocation`))
  (bind _returnvalue_2 (`GameplayStatics.GetPlayerCharacter` 0))
  (`NiagaraFunctionLibrary.SpawnSystemAtLocation` "/Game/TommasoContent/VFX/VFX_PlayerColorShot_Impact.VFX_PlayerColorShot_Impact" _returnvalue)
  (bind _returnvalue_3 (`GameplayStatics.GetActorOfClass` "/Game/MyContent/Blueprint/Enemies/BP_Enemy_Ranged.BP_Enemy_Ranged_C"))
  (bind _attackdamage (`/Game/MyContent/Blueprint/Enemies/BP_Enemy_Ranged.AttackDamage` _returnvalue_3))
  (`GameplayStatics.ApplyRadialDamage` :`BaseDamage` _attackdamage :`Origin` _returnvalue :`DamageRadius` 150.0 :`DamageCauser` null :`InstigatedByController` null)
  (if (<= (`self.GetDistanceTo` _returnvalue_2) 150.0)
    (`GameplayStatics.ApplyDamage` _returnvalue_2 _attackdamage))
  (`self.K2_DestroyActor`))

(fn `UserConstructionScript`)