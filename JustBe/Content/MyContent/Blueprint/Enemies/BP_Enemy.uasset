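; Base 2D Paper2D enemy character that patrols between two points and pursues the player once they enter its VisionZone.
; Tick drives movement, sprite facing and the walk flipbook, calling PerformAttack within AttackRange, which is an empty event here.
; Damage flashes the sprite red; death awards XP to BP_PlayerCharacter and destroys the actor.
; Aggro never clears, as the end-overlap event is empty and its reset logic is disconnected.
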(event `self.ReceiveTick`
  (params (DeltaSeconds :type "Float (single-precision)"))
  (bind _returnvalue_x (`KismetMathLibrary.BreakVector` (`self.K2_GetActorLocation`)))
  (bind _returnvalue_x_2 (`KismetMathLibrary.BreakVector` (`self.K2_GetActorLocation`)))
  (bind _returnvalue_x_3 (`KismetMathLibrary.BreakVector` (`self.K2_GetActorLocation` (`GameplayStatics.GetPlayerCharacter` 0))))
  (bind _returnvalue_x_4 (`KismetMathLibrary.BreakVector` (`self.K2_GetActorLocation` (`GameplayStatics.GetPlayerCharacter` 0))))
  (bind _returnvalue_x_5 (`KismetMathLibrary.BreakVector` (- (`self.CurrentTarget`) (`self.K2_GetActorLocation`))))
  (bind _returnvalue (`KismetMathLibrary.SignOfFloat` _returnvalue_x_5))
  (bind _returnvalue_2 (`KismetMathLibrary.SignOfFloat` (- _returnvalue_x_4 _returnvalue_x_2)))
  (if (`self.bIsAggro`)
    (`SceneComponent.SetRelativeScale3D` (`self.Sprite`) (`KismetMathLibrary.MakeVector` _returnvalue_2 1.0 1.0))
    (if (not (`self.bIsAttacking`))
      (if (< (`KismetMathLibrary.Abs` (- _returnvalue_x_3 _returnvalue_x)) (`self.AttackRange`))
        (`self.PerformAttack`)
        (else
          (set `CharacterMovementComponent.MaxWalkSpeed` 400.0 (`self.CharacterMovement`))
          (`self.AddMovementInput` (`KismetMathLibrary.MakeVector` _returnvalue_2))
          (`PaperFlipbookComponent.SetFlipbook` (`self.Sprite`) (`self.FlipbookWalk`)))))
    (else
      (`PaperFlipbookComponent.SetFlipbook` (`self.Sprite`) (`self.FlipbookWalk`))
      (set `CharacterMovementComponent.MaxWalkSpeed` (`self.PatrolSpeed`) (`self.CharacterMovement`))
      (`self.AddMovementInput` (`KismetMathLibrary.MakeVector` _returnvalue))
      (`SceneComponent.SetRelativeScale3D` (`self.Sprite`) (`KismetMathLibrary.MakeVector` _returnvalue 1.0 1.0))
      (if (<= (`KismetMathLibrary.Vector_Distance` (`self.K2_GetActorLocation`) (`self.CurrentTarget`)) 20.0)
        (if (== (`self.CurrentTarget`) (`self.PointA`))
          (set `self.CurrentTarget` (`self.PointB`))
          (else
            (set `self.CurrentTarget` (`self.PointA`))))))))

(event `self.ReceiveBeginPlay`
  (bind _returnvalue (`self.K2_GetActorLocation`))
  (set `self.CurrentHealth` (`self.MaxHealth`))
  (set `self.PointA` (+ _returnvalue (`self.PointA`)))
  (set `self.PointB` (+ _returnvalue (`self.PointB`)))
  (set `self.CurrentTarget` (`self.PointA`))
  (set `CharacterMovementComponent.MaxWalkSpeed` (`self.PatrolSpeed`) (`self.CharacterMovement`)))

(event `self.ReceiveAnyDamage`
  (params (Damage :type "Float (single-precision)") (DamageType :type "DamageType Object Reference") (InstigatedBy :type "Controller Object Reference") (DamageCauser :type "Actor Object Reference"))
  (bind _sprite (`self.Sprite`))
  (if (not (`self.bIsDead`))
    (set `self.CurrentHealth` (- (`self.CurrentHealth`) Damage))
    (`PaperFlipbookComponent.SetSpriteColor` _sprite (struct :`R` 0.605903 :`G` 0.045232 :`B` 0.045232 :`A` 1.0))
    (`KismetSystemLibrary.Delay` 0.1)
    (`PaperFlipbookComponent.SetSpriteColor` _sprite (struct :`R` 1.0 :`G` 1.0 :`B` 1.0 :`A` 1.0))
    (if (<= (`self.CurrentHealth`) 0.0)
      (`self.Die`))))

(event `Die`
  (set `self.bIsDead` true)
  (`PrimitiveComponent.SetCollisionEnabled` (`self.CapsuleComponent`) "NoCollision")
  (bind _asbp_player_character (cast `/Game/MyContent/Blueprint/BP_PlayerCharacter` (`GameplayStatics.GetPlayerCharacter` 0)))
  (`/Game/MyContent/Blueprint/BP_PlayerCharacter.AddXP` _asbp_player_character (`self.XPReward`))
  (`self.K2_DestroyActor`))

(event `self.VisionZone.OnComponentBeginOverlap`
  (params (OverlappedComponent :type "PrimitiveComponent Object Reference") (OtherActor :type "Actor Object Reference") (OtherComp :type "PrimitiveComponent Object Reference") (OtherBodyIndex :type Integer) (bFromSweep :type Boolean) (SweepResult :type "HitResult Structure (by ref)"))
  (cast `/Game/MyContent/Blueprint/BP_PlayerCharacter` OtherActor)
  (set `self.bIsAggro` true))

(event `self.VisionZone.OnComponentEndOverlap`
  (params (OverlappedComponent :type "PrimitiveComponent Object Reference") (OtherActor :type "Actor Object Reference") (OtherComp :type "PrimitiveComponent Object Reference") (OtherBodyIndex :type Integer)))

(event `PerformAttack`)

(fn `UserConstructionScript`)