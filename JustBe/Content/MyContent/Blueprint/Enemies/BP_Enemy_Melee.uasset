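; Melee enemy with flipbook sprites that attacks the player with a close-range slash and a periodic ground shockwave.
; PerformAttack shows a warning VFX, whose finish triggers the slash and a box trace toward the player that applies damage.
; A randomized timer spawns the shockwave at its feet when aggroed.
; Both attacks share an IsAttacking lock and skip dashing players, which also stops the shockwave timer from rescheduling.
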(event `self.ReceiveBeginPlay`
  (`parent.ReceiveBeginPlay`)
  (`self.CalculateNextGroundAttack`)
  (bind _asbp_player_character (cast `/Game/MyContent/Blueprint/BP_PlayerCharacter` (`GameplayStatics.GetPlayerCharacter` 0)))
  (set `self.PlayerRef` _asbp_player_character))

(event `CalculateNextGroundAttack`
  (`KismetSystemLibrary.K2_SetTimerDelegate` (delegate `PerformGroundAttack`) (`KismetMathLibrary.RandomFloatInRange` 5.0 7.0)))

(event `PerformGroundAttack`
  (bind (_returnvalue_x _returnvalue_y _returnvalue_z) (`KismetMathLibrary.BreakVector` (`self.K2_GetActorLocation`)))
  (bind _sprite (`self.Sprite`))
  (bind _relativescale3d_x (`KismetMathLibrary.BreakVector` (`SceneComponent.RelativeScale3D` (`self.Sprite`))))
  (if (and (`self.bIsAggro`) (not (`self.bIsAttacking`)))
    (if (not (`/Game/MyContent/Blueprint/BP_PlayerCharacter.bIsDashing` (`self.PlayerRef`)))
      (set `self.bIsAttacking` true)
      (`PaperFlipbookComponent.SetFlipbook` _sprite "/Game/MyContent/Sprites/FB_MeleeAbility.FB_MeleeAbility")
      (`PaperFlipbookComponent.SetLooping` _sprite false)
      (`PaperFlipbookComponent.PlayFromStart` _sprite)
      (`KismetSystemLibrary.Delay` 0.3)
      (`|SpawnActorFromClass` "/Game/MyContent/Blueprint/Enemies/MeleeAbility/BP_GroundShockwave.BP_GroundShockwave_C" (`KismetMathLibrary.MakeTransform` (`KismetMathLibrary.MakeVector` _returnvalue_x _returnvalue_y (- _returnvalue_z (`CapsuleComponent.GetScaledCapsuleHalfHeight` (`self.CapsuleComponent`)))) (select `bool` (< _relativescale3d_x 0.0) :`true` (`KismetMathLibrary.MakeRotator` 0.0 0.0 180.0))) "Undefined" "MultiplyWithRoot" null null)
      (`KismetSystemLibrary.Delay` (`self.AttackCooldown`))
      (set `self.bIsAttacking` false)
      (`self.CalculateNextGroundAttack`))
    (else
      (`self.CalculateNextGroundAttack`))))

(event `self.PerformAttack`
  (if (`/Game/MyContent/Blueprint/BP_PlayerCharacter.bIsDashing` (`self.PlayerRef`))
    _
    (elif (`NavMovementComponent.IsFalling` (`self.CharacterMovement`))
      _
      (elif (not (`self.bIsAttacking`))
        (set `self.bIsAttacking` true)
        (`PaperFlipbookComponent.Stop` (`self.Sprite`))
        (bind _returnvalue (`NiagaraFunctionLibrary.SpawnSystemAttached` "/Game/TommasoContent/VFX/VFX_EnemyAttackWarning.VFX_EnemyAttackWarning" (`self.Sprite`) "None" (0.0 0.0 50.0) (struct) "KeepRelativeOffset"))
        (add `NiagaraComponent.OnSystemFinished` _returnvalue (delegate `EnemyAttack`))))))

(event `EnemyAttack`
  (params (PSystem :type "NiagaraComponent Object Reference"))
  (bind (_returnvalue_x _returnvalue_y _returnvalue_z) (`KismetMathLibrary.BreakVector` (`self.K2_GetActorLocation`)))
  (bind _returnvalue_x_2 (`KismetMathLibrary.BreakVector` (`self.K2_GetActorLocation`)))
  (bind _sprite (`self.Sprite`))
  (bind _sprite_2 (`self.Sprite`))
  (bind _muzzle (`self.Muzzle`))
  (bind _returnvalue_x_3 (`KismetMathLibrary.BreakVector` (`self.K2_GetActorLocation` (`GameplayStatics.GetPlayerCharacter` 0))))
  (bind _returnvalue_x_4 (`KismetMathLibrary.BreakVector` (`self.K2_GetActorLocation` (`GameplayStatics.GetPlayerCharacter` 0))))
  (`PaperFlipbookComponent.SetFlipbook` _sprite_2 "/Game/MyContent/Sprites/FB_MeleeAttack.FB_MeleeAttack")
  (`PaperFlipbookComponent.SetLooping` _sprite_2 false)
  (`PaperFlipbookComponent.PlayFromStart` _sprite_2)
  (`SceneComponent.K2_SetRelativeRotation` _muzzle (`KismetMathLibrary.SelectRotator` (struct :`Yaw` 180.0) (struct) (< _returnvalue_x_4 _returnvalue_x_2)) false false)
  (`NiagaraFunctionLibrary.SpawnSystemAttached` "/Game/TommasoContent/VFX/VFX_EnemySlashAttack.VFX_EnemySlashAttack" _muzzle "None" (0.0 0.0 0.0) (struct) "SnapToTargetIncludingScale")
  (bind _outhit (`KismetSystemLibrary.BoxTraceSingle` (`self.K2_GetActorLocation`) (`KismetMathLibrary.MakeVector` (+ (* (`KismetMathLibrary.SignOfFloat` (- _returnvalue_x_3 _returnvalue_x)) (+ (`self.AttackRange`) 140.0)) _returnvalue_x) _returnvalue_y (+ _returnvalue_z 40.0)) (0.0 0.0 0.0) (struct) "TraceTypeQuery1"))
  (bind _asbp_player_character (cast `/Game/MyContent/Blueprint/BP_PlayerCharacter` (`.HitActor` (`GameplayStatics.BreakHitResult` _outhit)))
    (:`then`
      (`GameplayStatics.ApplyDamage` _asbp_player_character (`self.AttackDamage`))
      (`|ExecutionSequence`
        (:`then_0`
          (`KismetSystemLibrary.Delay` (`self.AttackCooldown`)))))
    (:`CastFailed`
      (`KismetSystemLibrary.Delay` (`PaperFlipbookComponent.GetFlipbookLength` _sprite))
      (`PaperFlipbookComponent.SetFlipbook` _sprite "/Game/MyContent/Sprites/Enemies/EnemyMelee/Walk/FB_MeleeWalk.FB_MeleeWalk")
      (`PaperFlipbookComponent.SetLooping` _sprite true)))
  (set `self.bIsAttacking` false))

(fn `UserConstructionScript`
  (`parent.UserConstructionScript`))