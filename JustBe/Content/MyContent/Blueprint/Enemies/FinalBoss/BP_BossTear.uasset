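; Final boss tear hazard that damages the player on contact and turns into shockwaves when it hits the ground.
; Its Hitbox hit event applies fixed damage to BP_PlayerCharacter, gated by a DoOnce, without destroying the tear.
; Other hits on a component or actor tagged Ground spawn two BP_BossShockwave actors at its location, one rotated 180 degrees, then destroy the tear.
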(event `self.ReceiveBeginPlay`)

(event `self.Hitbox.OnComponentHit`
  (params (HitComponent :type "PrimitiveComponent Object Reference") (OtherActor :type "Actor Object Reference") (OtherComp :type "PrimitiveComponent Object Reference") (NormalImpulse :type "Vector Structure") (Hit :type "HitResult Structure (by ref)"))
  (bind _returnvalue (`self.K2_GetActorLocation`))
  (bind _asbp_player_character (cast `/Game/MyContent/Blueprint/BP_PlayerCharacter` OtherActor)
    (:`then`
      (`/Engine/EditorBlueprintResources/StandardMacros.DoOnce` false
        (:`Completed`
          (`GameplayStatics.ApplyDamage` _asbp_player_character 15.0))))
    (:`CastFailed`
      (if (or (`ActorComponent.ComponentHasTag` OtherComp "Ground") (`self.ActorHasTag` OtherActor "Ground"))
        (`|SpawnActorFromClass` "/Game/MyContent/Blueprint/Enemies/MeleeAbility/BP_BossShockwave.BP_BossShockwave_C" (`KismetMathLibrary.MakeTransform` _returnvalue) "Undefined" "MultiplyWithRoot" null 40.0 null)
        (`|SpawnActorFromClass` "/Game/MyContent/Blueprint/Enemies/MeleeAbility/BP_BossShockwave.BP_BossShockwave_C" (`KismetMathLibrary.MakeTransform` _returnvalue (struct :`Yaw` 180.0)) "Undefined" "MultiplyWithRoot" null 40.0 null)
        (`self.K2_DestroyActor`)))))

(event `self.Hitbox.OnComponentBeginOverlap`
  (params (OverlappedComponent :type "PrimitiveComponent Object Reference") (OtherActor :type "Actor Object Reference") (OtherComp :type "PrimitiveComponent Object Reference") (OtherBodyIndex :type Integer) (bFromSweep :type Boolean) (SweepResult :type "HitResult Structure (by ref)")))

(fn `UserConstructionScript`)