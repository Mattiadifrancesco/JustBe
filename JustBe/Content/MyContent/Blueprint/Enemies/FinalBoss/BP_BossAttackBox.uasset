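; BP_BossAttackBox is a final boss attack projectile that damages the player once when its hitbox overlaps them.
; Overlapping a Ground-tagged actor triggers a behavior chosen by RoutineType.
; The side routines set horizontal projectile velocity left or right, then destroy the box after a short delay.
; The center routine spawns two opposite-facing BP_GroundShockwave actors and destroys the box immediately.
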(event `self.ReceiveBeginPlay`)

(event `self.Hitbox.OnComponentBeginOverlap`
  (params (OverlappedComponent :type "PrimitiveComponent Object Reference") (OtherActor :type "Actor Object Reference") (OtherComp :type "PrimitiveComponent Object Reference") (OtherBodyIndex :type Integer) (bFromSweep :type Boolean) (SweepResult :type "HitResult Structure (by ref)"))
  (bind _returnvalue (`self.K2_GetActorLocation`))
  (bind _asbp_player_character (cast `/Game/MyContent/Blueprint/BP_PlayerCharacter` OtherActor)
    (:`then`
      (`/Engine/EditorBlueprintResources/StandardMacros.DoOnce` false
        (:`Completed`
          (`GameplayStatics.ApplyDamage` _asbp_player_character 15.0))))
    (:`CastFailed`
      (if (`self.ActorHasTag` OtherActor "Ground")
        (switch `/Game/MyContent/Blueprint/Enemies/FinalBoss/E_RoutineType` (`self.RoutineType`)
          (:`NewEnumerator0`
            (set `MovementComponent.Velocity` (1200.0 0.0 0.0) (`self.ProjectileMovement`))
            (`KismetSystemLibrary.Delay` 1.0)
            (`self.K2_DestroyActor`))
          (:`NewEnumerator1`
            (`|SpawnActorFromClass` "/Game/MyContent/Blueprint/Enemies/MeleeAbility/BP_GroundShockwave.BP_GroundShockwave_C" (`KismetMathLibrary.MakeTransform` _returnvalue) "Undefined" "MultiplyWithRoot" null null)
            (`|SpawnActorFromClass` "/Game/MyContent/Blueprint/Enemies/MeleeAbility/BP_GroundShockwave.BP_GroundShockwave_C" (`KismetMathLibrary.MakeTransform` _returnvalue (struct :`Yaw` 180.0)) "Undefined" "MultiplyWithRoot" null null)
            (`self.K2_DestroyActor`))
          (:`NewEnumerator2`
            (set `MovementComponent.Velocity` (-1200.0 0.0 0.0) (`self.ProjectileMovement`))
            (`KismetSystemLibrary.Delay` 1.0)
            (`self.K2_DestroyActor`)))))))

(fn `UserConstructionScript`)