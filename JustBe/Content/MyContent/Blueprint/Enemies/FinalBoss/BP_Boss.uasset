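; Final boss actor with a Paper2D flipbook that alternates attack and vulnerability phases and is destroyed when health runs out.
; After an opening delay, it cycles between an invulnerable volley of attack boxes spawned above the player and an idle window with its hitbox enabled.
; At low health, checked between cycles, it stays vulnerable and repeatedly spawns tears from its center at random intervals.
; Damage flashes the sprite red; the timer-driven attack path is unused.
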(event `self.ReceiveBeginPlay`
  (`PaperFlipbookComponent.SetFlipbook` (`self.PaperFlipbook`) "/Game/MyContent/Sprites/Enemies/FinalBoss/FB_Attack.FB_Attack")
  (`PrimitiveComponent.SetCollisionEnabled` (`self.Hitbox`) "NoCollision")
  (`KismetSystemLibrary.Delay` 5.84)
  (`self.StartBossLoop`))

(event `StartBossLoop`
  (if (<= (`self.BossHealth`) 625.0)
    (`self.LowHpPhase`)
    (else
      (`self.InvulnerablePhase`))))

(event `InvulnerablePhase`
  (`PaperFlipbookComponent.SetFlipbook` (`self.PaperFlipbook`) "/Game/MyContent/Sprites/Enemies/FinalBoss/FB_Attack.FB_Attack")
  (`PrimitiveComponent.SetCollisionEnabled` (`self.Hitbox`) "NoCollision")
  (set `self.ContatoreAttacchi` (`KismetMathLibrary.RandomIntegerInRange` 3 7))
  (bind _output_get (set `self.AttackPatternIndex` 0))
  (switch `int` _output_get :!label _label
    (:`0`
      (`self.TopLeft`))
    (:`1`
      (`self.TopRight`))
    (:`2`
      (`self.Center`)))
  (`KismetSystemLibrary.Delay` 2.5)
  (bind _result (`/Engine/EditorBlueprintResources/StandardMacros.DecrementInt` (`self.ContatoreAttacchi`))
    (:`  `
      (if (> _result 0)
        (goto _label)
        (else
          (`self.VulnerablePhase`))))))

(event `VulnerablePhase`
  (`PaperFlipbookComponent.SetFlipbook` (`self.PaperFlipbook`) "/Game/MyContent/Sprites/Enemies/FinalBoss/FB_BossIdle.FB_BossIdle")
  (`PrimitiveComponent.SetCollisionEnabled` (`self.Hitbox`) "QueryOnly")
  (`KismetSystemLibrary.Delay` 3.5)
  (`self.StartBossLoop`))

(event `LowHpPhase`
  (`PaperFlipbookComponent.SetFlipbook` (`self.PaperFlipbook`) "/Game/MyContent/Sprites/Enemies/FinalBoss/FB_Idle2NDPHASE.FB_Idle2NDPHASE")
  (`PrimitiveComponent.SetCollisionEnabled` (`self.Hitbox`) "QueryOnly")
  (`KismetSystemLibrary.Delay` (`KismetMathLibrary.RandomFloatInRange` 1.0 4.0))
  (bind _output_get (set `self.AttackPatternIndex` 2))
  (switch `int` _output_get
    (:`0`
      (`self.TopLeft`))
    (:`1`
      (`self.TopRight`))
    (:`2`
      (`self.Center`)))
  (`self.LowHpPhase`))

(event `TopLeft`
  (bind _returnvalue (`SceneComponent.K2_GetComponentToWorld` (`self.SpawnTopLeft`)))
  (bind (_returnvalue_x _returnvalue_y _returnvalue_z) (`KismetMathLibrary.BreakVector` (`self.K2_GetActorLocation` (`GameplayStatics.GetPlayerCharacter` 0))))
  (`|SpawnActorFromClass` "/Game/MyContent/Blueprint/Enemies/FinalBoss/BP_BossAttackBox.BP_BossAttackBox_C" (`KismetMathLibrary.MakeTransform` (`KismetMathLibrary.MakeVector` _returnvalue_x _returnvalue_y (+ _returnvalue_z (.z (.location _returnvalue)))) (.rotation _returnvalue) (.scale _returnvalue)) "AdjustIfPossibleButAlwaysSpawn" "MultiplyWithRoot" null "NewEnumerator0" null)
  (`KismetSystemLibrary.Delay` 0.5))

(event `Center`
  (`|SpawnActorFromClass` "/Game/MyContent/Blueprint/Enemies/FinalBoss/BP_BossTear.BP_BossTear_C" (`SceneComponent.K2_GetComponentToWorld` (`self.SpawnCenter`)) "Undefined" "MultiplyWithRoot" null "NewEnumerator1" null))

(event `TopRight`
  (bind _returnvalue (`SceneComponent.K2_GetComponentToWorld` (`self.SpawnTopLeft`)))
  (bind (_returnvalue_x _returnvalue_y _returnvalue_z) (`KismetMathLibrary.BreakVector` (`self.K2_GetActorLocation` (`GameplayStatics.GetPlayerCharacter` 0))))
  (`|SpawnActorFromClass` "/Game/MyContent/Blueprint/Enemies/FinalBoss/BP_BossAttackBox.BP_BossAttackBox_C" (`KismetMathLibrary.MakeTransform` (`KismetMathLibrary.MakeVector` _returnvalue_x _returnvalue_y (+ _returnvalue_z (.z (.location _returnvalue)))) (.rotation _returnvalue) (.scale _returnvalue)) "AdjustIfPossibleButAlwaysSpawn" "MultiplyWithRoot" null "NewEnumerator2" null))

(event `StartBossAttack`
  (bind _returnvalue (`KismetSystemLibrary.K2_SetTimerDelegate` (delegate `ExecuteBossAttack`) (`KismetMathLibrary.RandomFloatInRange` 2.5 5.0)))
  (set `self.AttackTimerRef` _returnvalue))

(event `ExecuteBossAttack`
  (if (<= (`self.BossHealth`) 400.0)
    (`KismetSystemLibrary.PrintString` "Hello")
    (bind _output_get (set `self.AttackPatternIndex` 2))
    (switch `int` _output_get
      (:`0`
        (`self.TopLeft`))
      (:`1`
        (`self.TopRight`))
      (:`2`
        (`self.Center`)))
    (`self.StartBossAttack`)
    (else
      (bind _output_get_2 (set `self.AttackPatternIndex` (`KismetMathLibrary.RandomIntegerInRange` 0 1)))
      (switch `int` _output_get_2
        (:`0`
          (`self.TopLeft`))
        (:`1`
          (`self.TopRight`))
        (:`2`
          (`self.Center`)))
      (`self.StartBossAttack`))))

(event `self.ReceiveAnyDamage`
  (params (Damage :type "Float (single-precision)") (DamageType :type "DamageType Object Reference") (InstigatedBy :type "Controller Object Reference") (DamageCauser :type "Actor Object Reference"))
  (set `self.BossHealth` (- (`self.BossHealth`) Damage))
  (`PaperFlipbookComponent.SetSpriteColor` (`self.PaperFlipbook`) (struct :`R` 0.730461 :`A` 1.0))
  (`KismetSystemLibrary.Delay` 0.1)
  (`PaperFlipbookComponent.SetSpriteColor` (`self.PaperFlipbook`) (struct :`R` 1.0 :`G` 1.0 :`B` 1.0 :`A` 1.0))
  (if (<= (`self.BossHealth`) 0.0)
    (`self.K2_DestroyActor`)))

(fn `UserConstructionScript`)