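; Ranged 2D enemy that stops and lobs projectiles at the player while they are inside its vision zone.
; Entering the zone disables movement and starts a looping attack timer; leaving clears only the timer.
; Each attack flips the sprite toward the player, waits briefly, then spawns a projectile on a suggested arc aimed beyond the player's X position, with Y and Z zeroed.
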(event `self.VisionZone.OnComponentBeginOverlap`
  (params (OverlappedComponent :type "PrimitiveComponent Object Reference") (OtherActor :type "Actor Object Reference") (OtherComp :type "PrimitiveComponent Object Reference") (OtherBodyIndex :type Integer) (bFromSweep :type Boolean) (SweepResult :type "HitResult Structure (by ref)"))
  (cast `/Game/MyContent/Blueprint/BP_PlayerCharacter` OtherActor)
  (`CharacterMovementComponent.DisableMovement` (`self.CharacterMovement`))
  (set `self.bCanSeePlayer` true)
  (bind _returnvalue (`KismetSystemLibrary.K2_SetTimerDelegate` (delegate `PerformRangedAttack`) (`self.AttackSpeed`) true))
  (set `self.AttackTimerHandle` _returnvalue))

(event `PerformRangedAttack`
  (bind _returnvalue_x (`KismetMathLibrary.BreakVector` (`self.K2_GetActorLocation`)))
  (bind _muzzle (`self.Muzzle`))
  (bind _returnvalue (`SceneComponent.K2_GetComponentLocation` _muzzle))
  (bind _returnvalue_x_2 (`KismetMathLibrary.BreakVector` (`self.K2_GetActorLocation` (`GameplayStatics.GetPlayerCharacter` 0))))
  (bind _returnvalue_x_3 (`KismetMathLibrary.BreakVector` (`self.K2_GetActorLocation` (`GameplayStatics.GetPlayerCharacter` 0))))
  (`SceneComponent.SetRelativeScale3D` (`self.Sprite`) (`KismetMathLibrary.MakeVector` (`KismetMathLibrary.SignOfFloat` (- _returnvalue_x_3 _returnvalue_x)) 1.0 1.0))
  (`KismetSystemLibrary.Delay` 0.2)
  (bind _outlaunchvelocity (`GameplayStatics.SuggestProjectileVelocity_CustomArc` _returnvalue (`KismetMathLibrary.MakeVector` (+ (* (`KismetMathLibrary.SignOfFloat` (- _returnvalue_x_2 (.x _returnvalue))) 300.0) _returnvalue_x_2))))
  (bind _returnvalue_2 (`|SpawnActorFromClass` "/Game/MyContent/Blueprint/Enemies/RangedAbility/BP_EnemyRangedProjectile.BP_EnemyRangedProjectile_C" (`SceneComponent.K2_GetComponentToWorld` _muzzle) "Undefined" "MultiplyWithRoot" self null))
  (`PrimitiveComponent.IgnoreActorWhenMoving` (`/Game/MyContent/Blueprint/Enemies/RangedAbility/BP_EnemyRangedProjectile.Collision` _returnvalue_2) self false)
  (set `MovementComponent.Velocity` _outlaunchvelocity (`/Game/MyContent/Blueprint/Enemies/RangedAbility/BP_EnemyRangedProjectile.ProjectileMovement` _returnvalue_2)))

(event `self.VisionZone.OnComponentEndOverlap`
  (params (OverlappedComponent :type "PrimitiveComponent Object Reference") (OtherActor :type "Actor Object Reference") (OtherComp :type "PrimitiveComponent Object Reference") (OtherBodyIndex :type Integer))
  (cast `/Game/MyContent/Blueprint/BP_PlayerCharacter` OtherActor)
  (`KismetSystemLibrary.K2_ClearAndInvalidateTimerHandle` (`self.AttackTimerHandle`)))

(fn `UserConstructionScript`
  (`parent.UserConstructionScript`))