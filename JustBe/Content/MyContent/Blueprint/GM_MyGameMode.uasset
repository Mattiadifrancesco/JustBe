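; Game mode that tracks villager activation progress, handles saving and picks the player's spawn point.
; BeginPlay forces fullscreen at desktop resolution, then restores the villager count from the game instance, overridden by save slot "Slot1", which also restores the mask inventory.
; Each activation updates the game instance and fires colored and all-activated dispatchers.
; SaveGame writes progress to the slot; ChoosePlayerStart matches the last checkpoint tag, falling back to the first PlayerStart.
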(event `self.ReceiveBeginPlay`
  (bind _asgi_my_game_instance (cast `/Game/MyContent/Blueprint/Struct/GI_MyGameInstance` (`GameplayStatics.GetGameInstance`)))
  (set `self.ActivatedVillagersCount` (`/Game/MyContent/Blueprint/Struct/GI_MyGameInstance.ActivatedVillagers` _asgi_my_game_instance))
  (bind _returnvalue (`GameUserSettings.GetGameUserSettings`))
  (`GameUserSettings.SetScreenResolution` _returnvalue (`GameUserSettings.GetDesktopResolution` _returnvalue))
  (`GameUserSettings.SetFullscreenMode` _returnvalue "Fullscreen")
  (`GameUserSettings.ApplyResolutionSettings` _returnvalue false)
  (`GameUserSettings.SaveSettings` _returnvalue)
  (bind _asbp_player_character (cast `/Game/MyContent/Blueprint/BP_PlayerCharacter` (`GameplayStatics.GetPlayerCharacter` 0)))
  (set `self.PlayerRef` _asbp_player_character)
  (bind _returnvalue_2 (`GameplayStatics.DoesSaveGameExist` "Slot1"))
  (if _returnvalue_2
    (bind _returnvalue_3 (`GameplayStatics.LoadGameFromSlot` "Slot1"))
    (bind _asbp_save_game (cast `/Game/MyContent/Blueprint/SaveSystem/BP_SaveGame` _returnvalue_3))
    (set `self.ActivatedVillagersCount` (`/Game/MyContent/Blueprint/SaveSystem/BP_SaveGame.ActivatedVillagers` _asbp_save_game))
    (set `/Game/MyContent/Blueprint/BP_PlayerCharacter.MaskInventory` (`/Game/MyContent/Blueprint/SaveSystem/BP_SaveGame.UnclockedMasks` _asbp_save_game) (`self.PlayerRef`))
    (set `/Game/MyContent/Blueprint/SaveSystem/BP_SaveGame.ActivatedVillagerIDs` (`/Game/MyContent/Blueprint/SaveSystem/BP_SaveGame.ActivatedVillagerIDs` _asbp_save_game) _asbp_save_game)))

(event `OnVillagersActivated`
  (bind _result (`/Engine/EditorBlueprintResources/StandardMacros.IncrementInt` (`self.ActivatedVillagersCount`))
    (:`  `
      (bind _asgi_my_game_instance (cast `/Game/MyContent/Blueprint/Struct/GI_MyGameInstance` (`GameplayStatics.GetGameInstance`)))
      (set `/Game/MyContent/Blueprint/Struct/GI_MyGameInstance.ActivatedVillagers` _result _asgi_my_game_instance)
      (`self.OnVIllagerColored`)
      (if (>= _result (`self.TotalVillagersRequired`))
        (`self.OnAllVillagersActivated`)))))

(event `SaveGame`
  (bind _returnvalue (`GameplayStatics.DoesSaveGameExist` "Slot1"))
  (if _returnvalue
    (`GameplayStatics.LoadGameFromSlot` "Slot1")
    (else
      (bind _returnvalue_2 (`GameplayStatics.CreateSaveGameObject` "/Game/MyContent/Blueprint/SaveSystem/BP_SaveGame.BP_SaveGame_C"))))
  (bind _asbp_save_game (cast `/Game/MyContent/Blueprint/SaveSystem/BP_SaveGame` _returnvalue_2))
  (set `/Game/MyContent/Blueprint/SaveSystem/BP_SaveGame.ActivatedVillagers` (`self.ActivatedVillagersCount`) _asbp_save_game)
  (set `/Game/MyContent/Blueprint/SaveSystem/BP_SaveGame.UnclockedMasks` (`/Game/MyContent/Blueprint/BP_PlayerCharacter.MaskInventory` (`self.PlayerRef`)) _asbp_save_game)
  (set `/Game/MyContent/Blueprint/SaveSystem/BP_SaveGame.ActivatedVillagerIDs` (`/Game/MyContent/Blueprint/SaveSystem/BP_SaveGame.ActivatedVillagerIDs` _asbp_save_game) _asbp_save_game)
  (`GameplayStatics.SaveGameToSlot` null "Slot1"))

(fn `ChoosePlayerStart`
  (params (Player :type "Controller Object Reference"))
  (returns (ReturnValue :type "Actor Object Reference"))
  (bind _asgi_my_game_instance (cast `/Game/MyContent/Blueprint/Struct/GI_MyGameInstance` (`GameplayStatics.GetGameInstance`)))
  (bind _outactors (`GameplayStatics.GetAllActorsOfClass` "/Script/Engine.PlayerStart"))
  (for _array_element _outactors
    (if (== (`PlayerStart.PlayerStartTag` _array_element) (`/Game/MyContent/Blueprint/Struct/GI_MyGameInstance.LastCheckpointTag` _asgi_my_game_instance))
      (return _array_element)))
  (return (`|GetArrayItem` _outactors)))

(fn `UserConstructionScript`)