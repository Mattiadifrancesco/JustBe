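; BP_MaskPickup is a world pickup that grants its MaskToEquip to the player and shows a "mask obtained" screen.
; The construction script sets the sprite to the mask's idle flipbook, and DroppedMask gives TriggerZone an upward impulse.
; When an actor with BPC_MaskSystem overlaps TriggerZone, it adds the mask to player 0's inventory, saves it to the GameInstance, opens WBP_MaskObtained, pauses with UI-only input and destroys itself.
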(event `self.TriggerZone.OnComponentBeginOverlap`
  (params (OverlappedComponent :type "PrimitiveComponent Object Reference") (OtherActor :type "Actor Object Reference") (OtherComp :type "PrimitiveComponent Object Reference") (OtherBodyIndex :type Integer) (bFromSweep :type Boolean) (SweepResult :type "HitResult Structure (by ref)"))
  (bind _masktoequip (`self.MaskToEquip`))
  (`/Engine/EditorBlueprintResources/StandardMacros.IsValid` (`self.GetComponentByClass` OtherActor "/Game/MyContent/Blueprint/Struct/BPC_MaskSystem.BPC_MaskSystem_C")
    (:`Is Valid`
      (bind _asbp_player_character (cast `/Game/MyContent/Blueprint/BP_PlayerCharacter` (`GameplayStatics.GetPlayerCharacter` 0)))
      (`KismetArrayLibrary.Array_AddUnique` (`/Game/MyContent/Blueprint/BP_PlayerCharacter.MaskInventory` _asbp_player_character) _masktoequip)
      (`/Game/MyContent/Blueprint/BP_PlayerCharacter.SaveMaskToGI` _asbp_player_character)
      (bind _returnvalue (`|CreateWidget` "/Game/MyContent/Blueprint/UI/WBP_MaskObtained.WBP_MaskObtained_C" null (`KismetTextLibrary.Conv_NameToText` (`/Game/MyContent/Blueprint/Struct/PDA_MaskData.MaskName` _masktoequip)) (`/Game/MyContent/Blueprint/Struct/PDA_MaskData.DescrizioneUI` _masktoequip) (`/Game/MyContent/Blueprint/Struct/PDA_MaskData.MaskUIIcon` _masktoequip)))
      (`UserWidget.AddToViewport` _returnvalue 0)
      (`GameplayStatics.SetGamePaused` true)
      (`WidgetBlueprintLibrary.SetInputMode_UIOnlyEx` (`GameplayStatics.GetPlayerController` 0) _returnvalue)
      (`self.K2_DestroyActor`))))

(event `DroppedMask`
  (`/Engine/EditorBlueprintResources/StandardMacros.IsValid` (`self.MaskToEquip`)
    (:`Is Valid`
      (`PrimitiveComponent.AddImpulse` (`self.TriggerZone`) (0.0 0.0 100.0) "None" false))))

(fn `UserConstructionScript`
  (bind _masktoequip (`self.MaskToEquip`))
  (`/Engine/EditorBlueprintResources/StandardMacros.IsValid` _masktoequip
    (:`Is Valid`
      (`PaperFlipbookComponent.SetFlipbook` (`self.SpritePickup`) (`/Game/MyContent/Blueprint/Struct/PDA_MaskData.MaskFlipbook_Idle` _masktoequip)))))