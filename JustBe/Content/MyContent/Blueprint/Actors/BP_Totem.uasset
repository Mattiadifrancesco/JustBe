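; BP_Totem is an activatable totem that spends the player's collected colors to spread color through the world.
; Its trigger zone tracks player range and toggles a prompt widget until activation.
; LightUp checks BPCStats.CurrentLevel, deducts the cost, saves the player's transform as LastCheckpoint and removes the prompt.
; It writes the totem position to MPC_WorldColor, and a timeline expands the ColorRadius parameter from there.
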(event `self.TriggerZone.OnComponentBeginOverlap`
  (params (OverlappedComponent :type "PrimitiveComponent Object Reference") (OtherActor :type "Actor Object Reference") (OtherComp :type "PrimitiveComponent Object Reference") (OtherBodyIndex :type Integer) (bFromSweep :type Boolean) (SweepResult :type "HitResult Structure (by ref)"))
  (cast `/Game/MyContent/Blueprint/BP_PlayerCharacter` OtherActor)
  (set `self.bIsInRange` true)
  (if (not (`self.bIsPressed`))
    (`SceneComponent.SetVisibility` (`self.PromptWidget`) true false)))

(event `self.TriggerZone.OnComponentEndOverlap`
  (params (OverlappedComponent :type "PrimitiveComponent Object Reference") (OtherActor :type "Actor Object Reference") (OtherComp :type "PrimitiveComponent Object Reference") (OtherBodyIndex :type Integer))
  (cast `/Game/MyContent/Blueprint/BP_PlayerCharacter` OtherActor)
  (set `self.bIsInRange` false)
  (if (not (`self.bIsPressed`))
    (`SceneComponent.SetVisibility` (`self.PromptWidget`) false false)))

(event `LightUp`
  (params (PlayerRef :type "/Game/MyContent/Blueprint/BP_PlayerCharacter Object Reference"))
  (bind _bpc_stats (`/Game/MyContent/Blueprint/BP_PlayerCharacter.BPC_Stats` PlayerRef))
  (bind _colorstogive (`self.ColorsToGive`))
  (bind _currentlevel (`/Game/MyContent/Blueprint/Struct/BPC_Stats.CurrentLevel` _bpc_stats))
  (if (>= _currentlevel _colorstogive)
    (set `self.LastCheckpoint` (`SceneComponent.K2_GetComponentToWorld` (`Actor.RootComponent` (`GameplayStatics.GetPlayerCharacter` 0))))
    (set `/Game/MyContent/Blueprint/Struct/BPC_Stats.CurrentLevel` (- _currentlevel _colorstogive) _bpc_stats)
    (set `self.bIsPressed` true)
    (`ActorComponent.K2_DestroyComponent` (`self.PromptWidget`))
    (`KismetMaterialLibrary.SetVectorParameterValue` "/Game/MyContent/Blueprint/Materials/MPC_WorldColor.MPC_WorldColor" "TotemPosition" (`KismetMathLibrary.Conv_VectorToLinearColor` (`self.K2_GetActorLocation`)))
    (bind (_direction _alpha) (`Timeline|ExpandColor`)
      (:`Update`
        (`KismetMaterialLibrary.SetScalarParameterValue` "/Game/MyContent/Blueprint/Materials/MPC_WorldColor.MPC_WorldColor" "ColorRadius" (`KismetMathLibrary.Lerp` 0.0 35000.0 _alpha))))
    (else
      (`KismetSystemLibrary.PrintString` "servono 5 coloru"))))

(fn `UserConstructionScript`)