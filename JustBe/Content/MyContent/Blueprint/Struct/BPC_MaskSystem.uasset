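; BPC_MaskSystem is a player component that tracks the equipped mask and applies its look, stats and movement perk.
; EquipMask works as a toggle: the current mask again clears it, while a new one sets the mask flipbook, passes its data to BPC_Stats and broadcasts OnMaskChanged.
; Masks that grant color set custom depth stencil on both sprites.
; Dash Launcher allows a double jump; unequipping leaves jump count untouched.
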(fn `EquipMask`
  (params (NewMask :type "/Game/MyContent/Blueprint/Struct/PDA_MaskData Object Reference"))
  (bind _returnvalue (`KismetMathLibrary.SelectInt` 1 0 (`/Game/MyContent/Blueprint/Struct/PDA_MaskData.GrantsColor` NewMask)))
  (if (== (`self.CurrentMask`) NewMask)
    (bind _asbp_player_character (cast `/Game/MyContent/Blueprint/BP_PlayerCharacter` (`self.GetOwner`)))
    (`self.UnequipMask` (`/Game/MyContent/Blueprint/BP_PlayerCharacter.BPC_MaskSystem` _asbp_player_character))
    (`PrimitiveComponent.SetCustomDepthStencilValue` (`PaperCharacter.Sprite` _asbp_player_character) 0)
    (bind _masksprite (`/Game/MyContent/Blueprint/BP_PlayerCharacter.MaskSprite` _asbp_player_character))
    (`PrimitiveComponent.SetCustomDepthStencilValue` _masksprite 0)
    (`PaperFlipbookComponent.SetFlipbook` _masksprite null)
    (`/Game/MyContent/Blueprint/Struct/BPC_Stats.ApplyMaskStats` (`/Game/MyContent/Blueprint/BP_PlayerCharacter.BPC_Stats` _asbp_player_character) null)
    (else
      (bind _asbp_player_character_2 (cast `/Game/MyContent/Blueprint/BP_PlayerCharacter` (`self.GetOwner`)))
      (set `self.CurrentMask` NewMask)
      (`PrimitiveComponent.SetCustomDepthStencilValue` (`PaperCharacter.Sprite` _asbp_player_character_2) _returnvalue)
      (bind _masksprite_2 (`/Game/MyContent/Blueprint/BP_PlayerCharacter.MaskSprite` _asbp_player_character_2))
      (`PrimitiveComponent.SetCustomDepthStencilValue` _masksprite_2 _returnvalue)
      (`PaperFlipbookComponent.SetFlipbook` _masksprite_2 (`/Game/MyContent/Blueprint/Struct/PDA_MaskData.MaskFlipbook_Idle` NewMask))
      (`/Game/MyContent/Blueprint/Struct/BPC_Stats.ApplyMaskStats` (`Actor.GetComponentByClass` (`self.GetOwner`) "/Game/MyContent/Blueprint/Struct/BPC_Stats.BPC_Stats_C") NewMask)
      (switch `/Game/MyContent/Blueprint/Struct/E_MaskAbilityType` (`/Game/MyContent/Blueprint/Struct/PDA_MaskData.AbilityType` NewMask)
        (:`NewEnumerator0`
          (set `Character.JumpMaxCount` 2 _asbp_player_character_2))
        (:`NewEnumerator1`
          (set `Character.JumpMaxCount` 1 _asbp_player_character_2))
        (:`NewEnumerator2`
          (set `Character.JumpMaxCount` 1 _asbp_player_character_2))
        (:`NewEnumerator3`
          (set `Character.JumpMaxCount` 1 _asbp_player_character_2)))
      (`self.OnMaskChanged` NewMask))))

(fn `UnequipMask`
  (set `self.CurrentMask` null))