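; BPC_Stats is a component that holds a character's health, attack power, move speed and attack cooldown, and adjusts them for a mask.
; ApplyMaskStats adds the mask data's modifiers to base values, keeps the health percentage across max HP changes, and sets the player's walk speed.
; Without a valid mask it restores base attack, speed and cooldown values, but leaves max HP and the movement component's walk speed unchanged.
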(fn `ApplyMaskStats`
  (params (PDA_MaskData :type "/Game/MyContent/Blueprint/Struct/PDA_MaskData Object Reference"))
  (locals (LocalHealthPercentage :type "Float (double-precision)"))
  (bind _maxhp (`self.MaxHP`))
  (bind (_maxhealth _attackpower _movementspeed _attackspeed) (break `/Game/MyContent/Blueprint/Struct/ST_Stats` (`/Game/MyContent/Blueprint/Struct/PDA_MaskData.StatModifiers` PDA_MaskData)))
  (set `local.LocalHealthPercentage` (/ (`self.CurrentHealth`) (`self.MaxHP`)))
  (`/Engine/EditorBlueprintResources/StandardMacros.IsValid` PDA_MaskData
    (:`Is Valid`
      (bind _output_get (set `self.MaxHP` (+ (`self.BaseHealth`) _maxhealth)))
      (bind _output_get_2 (set `self.CurrentHealth` (`KismetMathLibrary.FClamp` (* (`local.LocalHealthPercentage`) _output_get) 0.0 (`self.MaxHP`))))
      (`KismetSystemLibrary.PrintString` (`KismetStringLibrary.Conv_DoubleToString` _output_get_2))
      (set `self.CurrentAttackPower` (+ _attackpower (`self.BaseAttackPower`)))
      (set `self.CurrentMoveSpeed` (+ _movementspeed (`self.BaseMoveSpeed`)))
      (set `self.CurrentAttackCooldown` (+ _attackspeed (`self.BaseAttackCooldown`)))
      (bind _asbp_player_character (cast `/Game/MyContent/Blueprint/BP_PlayerCharacter` (`self.GetOwner`)))
      (set `CharacterMovementComponent.MaxWalkSpeed` (`self.CurrentMoveSpeed`) (`Character.CharacterMovement` _asbp_player_character)))
    (:`Is Not Valid`
      (set `self.CurrentAttackPower` (`self.BaseAttackPower`))
      (set `self.CurrentMoveSpeed` (`self.BaseMoveSpeed`))
      (set `self.CurrentAttackCooldown` (`self.BaseAttackCooldown`))
      (set `self.CurrentHealth` (`KismetMathLibrary.FClamp` (* (`local.LocalHealthPercentage`) _maxhp) 0.0 _maxhp)))))