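; Test player character for a 2D side-scroller with flipbook animation, side movement, jumping and directional box-trace slash attacks.
; The current mask sets attack delay and selects the ability: a swept timeline dash that launches the struck enemy, or a delayed radial-damage bomb.
; Attacks and dashes drain timer-regenerated stamina, while timelines drive HUD cooldowns.
; It also handles XP levelling, totem interaction, pausing, and quitting the game on death.
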(event `self.ReceiveTick`
  (params (DeltaSeconds :type "Float (single-precision)"))
  (bind _vfx_footdusttrail (`self.VFX_FootDustTrail`))
  (`self.UpdateAnimation`)
  (if (> (`KismetMathLibrary.VSize` (`self.GetVelocity`)) 1.0)
    (if (`NavMovementComponent.IsFalling` (`self.CharacterMovement`))
      (`ActorComponent.Deactivate` _vfx_footdusttrail :!label _label)
      (else
        (`ActorComponent.Activate` _vfx_footdusttrail false)))
    (else
      (goto _label))))

(event `self.ReceiveBeginPlay`
  (bind _bpc_stats (`self.BPC_Stats`))
  (`EnhancedInputSubsystemInterface.AddMappingContext` (pcsubsystem `EnhancedInputLocalPlayerSubsystem` (`GameplayStatics.GetPlayerController` 0)) "/Game/MyContent/Input/IMC_MainCharacter.IMC_MainCharacter" 0 (struct))
  (bind _returnvalue (`|CreateWidget` "/Game/MyContent/Blueprint/UI/WBP_HUD.WBP_HUD_C"))
  (bind _output_get (set `self.HUDRef` _returnvalue))
  (`UserWidget.AddToViewport` _output_get 0)
  (`/Game/MyContent/Blueprint/UI/WBP_HUD.UpdateXPUI` _output_get (`/Game/MyContent/Blueprint/Struct/BPC_Stats.CurrentXP` _bpc_stats) (`/Game/MyContent/Blueprint/Struct/BPC_Stats.MaxXP` _bpc_stats) (`KismetMathLibrary.FTrunc` (`/Game/MyContent/Blueprint/Struct/BPC_Stats.CurrentLevel` _bpc_stats)))
  (set `/Game/MyContent/Blueprint/Struct/BPC_Stats.CurrentLevel` 0.0 (`self.BPC_Stats`))
  (for _array_element (`self.AllMasks`)
    (set `/Game/MyContent/Blueprint/Struct/PDA_MaskData.UpgradeLevel` 1 _array_element)
    (set `/Game/MyContent/Blueprint/Struct/PDA_MaskData.StatModifiers` (make `/Game/MyContent/Blueprint/Struct/ST_Stats` (`/Game/MyContent/Blueprint/Struct/PDA_MaskData.BaseMaxHealth` _array_element) (`/Game/MyContent/Blueprint/Struct/PDA_MaskData.BaseAttackPower` _array_element) (`/Game/MyContent/Blueprint/Struct/PDA_MaskData.BaseMovementSpeed` _array_element) (`/Game/MyContent/Blueprint/Struct/PDA_MaskData.BaseAttackSpeed` _array_element) (`/Game/MyContent/Blueprint/Struct/PDA_MaskData.BaseDefense` _array_element)) _array_element)))

(event `EnhancedInput|/Game/MyContent/Input/Actions/IA_Move`
  (params (ActionValue :type "Float (double-precision)") (ElapsedSeconds :type "Float (double-precision)") (TriggeredSeconds :type "Float (double-precision)") (InputAction :type "InputAction Object Reference" :default "/Game/MyContent/Input/Actions/IA_Move.IA_Move"))
  (:`Triggered`
    (`self.AddMovementInput` (1.0 0.0 0.0) ActionValue)
    (if (> ActionValue 0.0)
      (`SceneComponent.SetRelativeScale3D` (`self.Sprite`) (1.0 1.0 1.0))
      (`SceneComponent.K2_SetRelativeRotation` :`self` (`self.VFX_FootDustTrail`))
      (elif (< ActionValue 0.0)
        (`SceneComponent.SetRelativeScale3D` (`self.Sprite`) (-1.0 1.0 1.0))
        (`SceneComponent.K2_SetRelativeRotation` (`self.VFX_FootDustTrail`) (struct :`Yaw` 180.0) false false)))))

(event `EnhancedInput|/Game/MyContent/Input/Actions/IA_Jump`
  (params (ActionValue :type Boolean) (ElapsedSeconds :type "Float (double-precision)") (TriggeredSeconds :type "Float (double-precision)") (InputAction :type "InputAction Object Reference" :default "/Game/MyContent/Input/Actions/IA_Jump.IA_Jump"))
  (:`Started`
    (`self.Jump`))
  (:`Completed`
    (`self.StopJumping`)))

(event `EnhancedInput|/Game/MyContent/Input/Actions/IA_VerticalAttack`
  (params (ActionValue :type "Float (double-precision)") (ElapsedSeconds :type "Float (double-precision)") (TriggeredSeconds :type "Float (double-precision)") (InputAction :type "InputAction Object Reference" :default "/Game/MyContent/Input/Actions/IA_VerticalAttack.IA_VerticalAttack"))
  (:`Triggered`
    (set `self.VerticalInput` ActionValue))
  (:`Completed`
    (set `self.VerticalInput` 0.0)))

(event `EnhancedInput|/Game/MyContent/Input/Actions/IA_Attack`
  (params (ActionValue :type Boolean) (ElapsedSeconds :type "Float (double-precision)") (TriggeredSeconds :type "Float (double-precision)") (InputAction :type "InputAction Object Reference" :default "/Game/MyContent/Input/Actions/IA_Attack.IA_Attack"))
  (bind _sprite (`self.Sprite`))
  (bind _currentmask (`/Game/MyContent/Blueprint/Struct/BPC_MaskSystem.CurrentMask` (`self.BPC_MaskSystem`)))
  (bind (_statmodifiers_maxhealth _statmodifiers_attackpower _statmodifiers_movementspeed _statmodifiers_attackspeed) (break `/Game/MyContent/Blueprint/Struct/ST_Stats` (`/Game/MyContent/Blueprint/Struct/PDA_MaskData.StatModifiers` _currentmask)))
  (:`Started`
    (if (`self.bCanAttack`)
      (if (not (<= (`/Game/MyContent/Blueprint/Struct/BPC_Stats.CurrentStamina` (`self.BPC_Stats`)) 4.0))
        (`self.ConsumeStaminaAndPauseRegen` 5.0)
        (`|ExecutionSequence`
          (:`then_0`
            (set `self.bIsAttacking` true)
            (set `self.bCanAttack` false)
            (if (> (`self.VerticalInput`) 0.3)
              (`self.PerformAttack` (0.0 0.0 120.0) (struct :`Pitch` 90.0))
              (`PaperFlipbookComponent.SetFlipbook` _sprite (`self.FB_AttackUP`))
              (elif (< (`self.VerticalInput`) -0.3)
                (`self.PerformAttack` (0.0 0.0 -100.0) (struct :`Pitch` -90.0))
                (`PaperFlipbookComponent.SetFlipbook` _sprite (`self.FB_AttackDown`))
                (else
                  (`self.PerformAttack` (100.0 0.0 0.0))
                  (`PaperFlipbookComponent.SetFlipbook` _sprite (`self.FB_Attack`)))))
            (`/Engine/EditorBlueprintResources/StandardMacros.IsValid` _currentmask
              (:`Is Valid`
                (`KismetSystemLibrary.Delay` _statmodifiers_attackspeed))
              (:`Is Not Valid`
                (`KismetSystemLibrary.Delay` 0.35)))
            (set `self.bCanAttack` true))
          (:`then_1`
            (`KismetSystemLibrary.Delay` (`PaperFlipbook.GetTotalDuration` (`self.FB_Attack`)))
            (set `self.bIsAttacking` false)))))))

(event `EnhancedInput|/Game/MyContent/Input/Actions/IA_Ability`
  (params (ActionValue :type Boolean) (ElapsedSeconds :type "Float (double-precision)") (TriggeredSeconds :type "Float (double-precision)") (InputAction :type "InputAction Object Reference" :default "/Game/MyContent/Input/Actions/IA_Ability.IA_Ability"))
  (bind _currentmask (`/Game/MyContent/Blueprint/Struct/BPC_MaskSystem.CurrentMask` (`self.BPC_MaskSystem`)))
  (:`Started`
    (`/Engine/EditorBlueprintResources/StandardMacros.IsValid` _currentmask
      (:`Is Valid`
        (switch `/Game/MyContent/Blueprint/Struct/E_MaskAbilityType` (`/Game/MyContent/Blueprint/Struct/PDA_MaskData.AbilityType` _currentmask)
          (:`NewEnumerator0`
            (if (`self.bCanDoDash`)
              (`self.ExecuteDashLauncher`)))
          (:`NewEnumerator1`
            (if (`self.bCanPerformBomb`)
              (set `self.bCanPerformBomb` false)
              (`Controller.SetIgnoreMoveInput` (`GameplayStatics.GetPlayerController` 0) true)
              (`KismetSystemLibrary.Delay` 1.0)
              (`self.PerformBomb`)
              (bind (_direction _percent) (`Timeline|BombCooldown` :!via `PlayFromStart`)
                (:`Update`
                  (`MaterialInstanceDynamic.SetScalarParameterValue` (`/Game/MyContent/Blueprint/UI/WBP_HUD.CooldownMaterialRef` (`self.HUDRef`)) "Percent" _percent))
                (:`Finished`
                  (set `self.bCanPerformBomb` true))))))))))

(event `ExecuteDashLauncher`
  (bind _returnvalue (`self.K2_GetActorLocation`))
  (bind _relativescale3d_x (`KismetMathLibrary.BreakVector` (`SceneComponent.RelativeScale3D` (`self.Sprite`))))
  (bind _returnvalue_2 (`KismetMathLibrary.MakeVector` _relativescale3d_x))
  (if (not (<= (`/Game/MyContent/Blueprint/Struct/BPC_Stats.CurrentStamina` (`self.BPC_Stats`)) 19.0))
    (set `self.bCanDoDash` false)
    (`self.ConsumeStaminaAndPauseRegen` 20.0)
    (set `self.bIsDashing` true)
    (`NiagaraFunctionLibrary.SpawnSystemAttached` "/Game/TommasoContent/VFX/VFX_DashTrail.VFX_DashTrail" (`self.CapsuleComponent`) "None" (0.0 0.0 0.0) (struct) "SnapToTarget" true)
    (set `self.bHasHitEnemy` false)
    (bind _output_get (set `self.DashStartLocation` (`self.K2_GetActorLocation`)))
    (set `self.DashDirection` _returnvalue_2)
    (set `self.DashEndLocation` (+ _output_get (* _returnvalue_2 (`self.AbilityDashLength`))))
    (bind (_direction _alpha) (`Timeline|TL_Dash` :!via `PlayFromStart`)
      (:`Update`
        (`self.K2_SetActorLocation` (`KismetMathLibrary.VLerp` (`self.DashStartLocation`) (`self.DashEndLocation`) _alpha) true)
        (bind _outhit (`KismetSystemLibrary.BoxTraceSingle` _returnvalue (+ _returnvalue (* (`self.DashDirection`) 20.0)) (30.0 30.0 60.0) (struct) "TraceTypeQuery1"))
        (bind _asbp_enemy (cast `/Game/MyContent/Blueprint/Enemies/BP_Enemy` (`.HitActor` (`GameplayStatics.BreakHitResult` _outhit)))
          (:`then`
            (if (not (`self.bHasHitEnemy`))
              (set `self.bHasHitEnemy` true)
              (`TimelineComponent.Stop` (`self.TL_Dash`))
              (`GameplayStatics.ApplyDamage` _asbp_enemy (`self.AbilityDashDamage`))
              (`self.LaunchCharacter` (0.0 0.0 1000.0) true true)
              (`self.LaunchCharacter` _asbp_enemy (0.0 0.0 800.0) false true)
              (set `self.bIsDashing` false)
              (else
                (bind (_direction_2 _percent) (`Timeline|Timeline` :!via `PlayFromStart` :!label _label_2)
                  (:`Update`
                    (`MaterialInstanceDynamic.SetScalarParameterValue` (`/Game/MyContent/Blueprint/UI/WBP_HUD.CooldownMaterialRef` (`self.HUDRef`)) "Percent" _percent))
                  (:`Finished`
                    (set `self.bCanDoDash` true))))))
          (:`CastFailed`
            (goto _label_2 :!via `PlayFromStart`))))
      (:`Finished`
        (set `self.bIsDashing` false)))))

(event `StartStaminaRegene`
  (bind _returnvalue (`KismetSystemLibrary.K2_SetTimerDelegate` (delegate `RegenStamina`) 0.1 true))
  (set `self.StaminaTimerHandle` _returnvalue))

(event `RegenStamina`
  (bind _bpc_stats (`self.BPC_Stats`))
  (bind _currentstamina (`/Game/MyContent/Blueprint/Struct/BPC_Stats.CurrentStamina` _bpc_stats))
  (bind _maxstamina (`/Game/MyContent/Blueprint/Struct/BPC_Stats.MaxStamina` _bpc_stats))
  (if (< _currentstamina _maxstamina)
    (set `/Game/MyContent/Blueprint/Struct/BPC_Stats.CurrentStamina` (`KismetMathLibrary.FClamp` (+ _currentstamina 1.0) 0.0 _maxstamina) _bpc_stats)
    (else
      (`KismetSystemLibrary.K2_ClearAndInvalidateTimerHandle` (`self.StaminaTimerHandle`)))))

(event `ConsumeStaminaAndPauseRegen`
  (params (StaminaToConsume :type "Float (double-precision)"))
  (bind _bpc_stats (`self.BPC_Stats`))
  (set `/Game/MyContent/Blueprint/Struct/BPC_Stats.CurrentStamina` (- (`/Game/MyContent/Blueprint/Struct/BPC_Stats.CurrentStamina` _bpc_stats) StaminaToConsume) _bpc_stats)
  (`KismetSystemLibrary.K2_ClearAndInvalidateTimerHandle` (`self.StaminaTimerHandle`))
  (`KismetSystemLibrary.Delay` 1.0)
  (`self.StartStaminaRegene`))

(event `AddXP`
  (params (XPAmount :type "Float (double-precision)"))
  (bind _bpc_stats (`self.BPC_Stats`))
  (bind _bpc_stats_2 (`self.BPC_Stats`))
  (bind _maxxp (`/Game/MyContent/Blueprint/Struct/BPC_Stats.MaxXP` _bpc_stats_2))
  (bind _output_get (set `self.TotalXP` (+ XPAmount (`/Game/MyContent/Blueprint/Struct/BPC_Stats.CurrentXP` _bpc_stats))))
  (while (>= _output_get (`/Game/MyContent/Blueprint/Struct/BPC_Stats.MaxXP` _bpc_stats))
    (set `/Game/MyContent/Blueprint/Struct/BPC_Stats.CurrentExp` (- (`self.TotalXP`) (`/Game/MyContent/Blueprint/Struct/BPC_Stats.MaxXP` _bpc_stats_2)) _bpc_stats_2)
    (set `/Game/MyContent/Blueprint/Struct/BPC_Stats.CurrentLevel` (+ (`/Game/MyContent/Blueprint/Struct/BPC_Stats.CurrentLevel` _bpc_stats_2) 1.0) _bpc_stats_2)
    (bind _output_get_2 (set `/Game/MyContent/Blueprint/Struct/BPC_Stats.MaxXP` (* _maxxp 1.2) _bpc_stats_2))
    (set `self.TotalXP` (- (`self.TotalXP`) _maxxp))
    (`/Game/MyContent/Blueprint/UI/WBP_HUD.UpdateXPUI` (`self.HUDRef`) (stale _output_get_3) _output_get_2 (`KismetMathLibrary.FTrunc` (`/Game/MyContent/Blueprint/Struct/BPC_Stats.CurrentLevel` _bpc_stats))))
  (bind _output_get_3 (set `/Game/MyContent/Blueprint/Struct/BPC_Stats.CurrentExp` (`self.TotalXP`) (`self.BPC_Stats`))))

(event `self.ReceiveAnyDamage`
  (params (Damage :type "Float (single-precision)") (DamageType :type "DamageType Object Reference") (InstigatedBy :type "Controller Object Reference") (DamageCauser :type "Actor Object Reference"))
  (bind _bpc_stats (`self.BPC_Stats`))
  (bind _output_get (set `/Game/MyContent/Blueprint/Struct/BPC_Stats.CurrentHealth` (- (`/Game/MyContent/Blueprint/Struct/BPC_Stats.CurrentHealth` _bpc_stats) Damage) _bpc_stats))
  (`self.Death` _output_get))

(event `EnhancedInput|/Game/MyContent/Input/Actions/IA_PauseGame`
  (params (ActionValue :type Boolean) (ElapsedSeconds :type "Float (double-precision)") (TriggeredSeconds :type "Float (double-precision)") (InputAction :type "InputAction Object Reference" :default "/Game/MyContent/Input/Actions/IA_PauseGame.IA_PauseGame"))
  (bind _returnvalue (`GameplayStatics.GetPlayerController` 0))
  (:`Started`
    (bind _returnvalue_2 (`|CreateWidget` "/Game/MyContent/Blueprint/UI/WBP_PauseMenu.WBP_PauseMenu_C"))
    (bind _output_get (set `self.PauseMenuRef` _returnvalue_2))
    (`UserWidget.AddToViewport` _output_get 0)
    (`GameplayStatics.SetGamePaused` true)
    (`WidgetBlueprintLibrary.SetInputMode_GameAndUIEx` _returnvalue _output_get)
    (set `PlayerController.bShowMouseCursor` true _returnvalue)))

(event `EnhancedInput|/Game/Variant_SideScroller/Input/Actions/IA_Interact`
  (params (ActionValue :type Boolean) (ElapsedSeconds :type "Float (double-precision)") (TriggeredSeconds :type "Float (double-precision)") (InputAction :type "InputAction Object Reference" :default "/Game/Variant_SideScroller/Input/Actions/IA_Interact.IA_Interact"))
  (bind _bpc_stats (`self.BPC_Stats`))
  (:`Started`
    (bind _returnvalue (`GameplayStatics.GetActorOfClass` "/Game/MyContent/Blueprint/Actors/BP_Totem.BP_Totem_C"))
    (if (`/Game/MyContent/Blueprint/Actors/BP_Totem.bIsInRange` _returnvalue)
      (if (not (`/Game/MyContent/Blueprint/Actors/BP_Totem.bIsPressed` _returnvalue))
        (`/Game/MyContent/Blueprint/Actors/BP_Totem.LightUp` _returnvalue self)
        (`/Game/MyContent/Blueprint/UI/WBP_HUD.UpdateXPUI` (`self.HUDRef`) (`/Game/MyContent/Blueprint/Struct/BPC_Stats.CurrentExp` _bpc_stats) (`/Game/MyContent/Blueprint/Struct/BPC_Stats.MaxXP` _bpc_stats) (`KismetMathLibrary.FTrunc` (`/Game/MyContent/Blueprint/Struct/BPC_Stats.CurrentLevel` _bpc_stats)))
        (else
          (bind _returnvalue_2 (`|CreateWidget` "/Game/MyContent/Blueprint/UI/WBP_TotemMenu.WBP_TotemMenu_C"))
          (`UserWidget.AddToViewport` _returnvalue_2 0))))))

(fn `Death`
  (params (Health :type "Float (double-precision)"))
  (if (<= Health 0.0)
    (`KismetSystemLibrary.QuitGame` null "Quit")))

(fn `PerformAttack`
  (params (AttackOffset :type "Vector Structure") (VFXRotation :type "Rotator Structure"))
  (bind _relativescale3d_x (`KismetMathLibrary.BreakVector` (`SceneComponent.RelativeScale3D` (`self.Sprite`))))
  (bind _output_get (set `self.HitLocation` (+ (`KismetMathLibrary.MakeVector` (* (.x AttackOffset) _relativescale3d_x) (.y AttackOffset) (.z AttackOffset)) (`self.K2_GetActorLocation`))))
  (bind _returnvalue (`NiagaraFunctionLibrary.SpawnSystemAtLocation` "/Game/TommasoContent/VFX/VFX_SlashAttack.VFX_SlashAttack" _output_get (`KismetMathLibrary.ComposeRotators` VFXRotation (select `bool` (< _relativescale3d_x 0.0) :`false` (`KismetMathLibrary.MakeRotator` 0.0) :`true` (`KismetMathLibrary.MakeRotator` 0.0 0.0 180.0)))))
  (`PrimitiveComponent.SetRenderCustomDepth` _returnvalue true)
  (`PrimitiveComponent.SetCustomDepthStencilValue` _returnvalue 1)
  (bind (_outhit _returnvalue_2) (`KismetSystemLibrary.BoxTraceSingle` _output_get _output_get (150.0 150.0 50.0) VFXRotation "TraceTypeQuery1"))
  (for _array_element (`|MakeArray` _outhit)
    (if _returnvalue_2
      (bind (_bblockinghit _binitialoverlap _time _distance _location _impactpoint _normal _impactnormal _physmat _hitactor) (`GameplayStatics.BreakHitResult` _array_element))
      (bind _asbp_enemy (cast `/Game/MyContent/Blueprint/Enemies/BP_Enemy` _hitactor))
      (`GameplayStatics.ApplyDamage` _hitactor (`/Game/MyContent/Blueprint/Struct/BPC_Stats.CurrentAttackPower` (`self.BPC_Stats`)) (`GameplayStatics.GetPlayerController` 0) self)
      (`NiagaraFunctionLibrary.SpawnSystemAtLocation` "/Game/TommasoContent/VFX/VFX_BrushImpact.VFX_BrushImpact" (`SceneComponent.K2_GetComponentLocation` (`PaperCharacter.Sprite` _asbp_enemy))))))

(fn `PerformBomb`
  (bind _returnvalue (`GameplayStatics.GetPlayerController` 0))
  (bind _returnvalue_2 (`self.K2_GetActorLocation`))
  (`NiagaraFunctionLibrary.SpawnSystemAttached` null (`self.CapsuleComponent`) "None" (0.0 0.0 0.0) (struct) "KeepRelativeOffset")
  (`GameplayStatics.ApplyRadialDamage` :`BaseDamage` 101.0 :`Origin` _returnvalue_2 :`DamageRadius` 400.0 :`DamageCauser` self :`InstigatedByController` _returnvalue :`bDoFullDamage` true :`DamagePreventionChannel` "ECC_Pawn")
  (`KismetSystemLibrary.DrawDebugSphere` _returnvalue_2 400.0 12 (struct :`R` 1.0 :`G` 1.0 :`B` 1.0 :`A` 1.0) 2.0)
  (`Controller.SetIgnoreMoveInput` _returnvalue false))

(fn `UpdateAnimation`
  (if (`self.bIsDashing`)
    (`PaperFlipbookComponent.SetFlipbook` (`self.Sprite`) (`self.FB_Dash`))
    (elif (`self.bIsAttacking`)
      _
      (elif (`NavMovementComponent.IsFalling` (`self.CharacterMovement`))
        (`PaperFlipbookComponent.SetFlipbook` (`self.Sprite`) (`self.FB_Jump`))
        (elif (> (`KismetMathLibrary.VSize` (`self.GetVelocity`)) 10.0)
          (`PaperFlipbookComponent.SetFlipbook` (`self.Sprite`) (`self.FB_Run`))
          (else
            (`PaperFlipbookComponent.SetFlipbook` (`self.Sprite`) (`self.FB_Idle`))))))))

(fn `UserConstructionScript`)